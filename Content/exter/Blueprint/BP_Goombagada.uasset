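; BP_Goombagada is a stompable enemy that hurts the player on contact.
; A head hitbox overlap disables itself, bounces the player (velocity depends on Space being held), plays a stomp sound and destroys the enemy unless Invincible.
; The body hitbox calls Hit on the character and knocks it away.
; Stomp deaths and Tick-detected falls below water level notify the active BP_ArenaTriggerErwan, if exactly one trigger exists.
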(event OnComponentBeginOverlap(headhitbox)
  (params (OverlappedComponent :type Primitive%20Component%20Object%20Reference) (OtherActor :type Actor%20Object%20Reference) (OtherComp :type Primitive%20Component%20Object%20Reference) (OtherBodyIndex :type Integer) (bFromSweep :type Boolean) (SweepResult :type Hit%20Result%20Structure%20%28by%20ref%29))
  (Utilities|Casting|CastToThirdPersonCharacter OtherActor)
  (Collision|SetCollisionEnabled (Variables|Default|Getheadhitbox) "NoCollision")
  (if (Game|Player|IsInputKeyDown (Game|GetPlayerController 0) "SpaceBar")
    (Variables|Default|SetjumpVelocity (Variables|Default|GetSpaceJump))
    (else
      (Variables|Default|SetjumpVelocity (Variables|Default|GetNoSpaceJump))))
  (Character|LaunchCharacter (Game|GetPlayerCharacter 0) (Variables|Default|GetjumpVelocity) false true)
  (Audio|PlaySound2D "/Game/exter/Audio/A_Goombagada_Stomp.A_Goombagada_Stomp" 1.0 1.0 0.0 0 0)
  (if (not (Variables|Default|GetInvincible))
    (Actor|DestroyActor)
    (CallFunction|DestroyinArena)))

(event OnComponentBeginOverlap(HitBox)
  (params (OverlappedComponent :type Primitive%20Component%20Object%20Reference) (OtherActor :type Actor%20Object%20Reference) (OtherComp :type Primitive%20Component%20Object%20Reference) (OtherBodyIndex :type Integer) (bFromSweep :type Boolean) (SweepResult :type Hit%20Result%20Structure%20%28by%20ref%29))
  (bind _returnvalue (Game|GetPlayerCharacter 0))
  (bind _asthird_person_character (Utilities|Casting|CastToThirdPersonCharacter OtherActor))
  (Default|Hit _asthird_person_character)
  (Character|LaunchCharacter _returnvalue (* (Math|Vector|Normalize (- (Transformation|GetWorldLocation (Variables|/Script/Engine.Actor|GetRootComponent _returnvalue)) (Transformation|GetWorldLocation (Variables|Collision|GetCapsuleComponent)))) 3.5e+03) true true))

(event EventTick
  (params (DeltaSeconds :type Float%20%28single-precision%29))
  ;[1 1 1] Enemy falling into water
  (if (< (.Z (Math|Vector|BreakVector (Transformation|GetWorldLocation (Variables|Character|GetMesh)))) -2e+01)
    (Actor|DestroyActor)
    (CallFunction|DestroyinArena)))

(fn ConstructionScript)

(fn DestroyinArena
  ;[1 1 1] Call DecrementEnemies function to know if thre are any enemies remaining in the arena
  (bind _outactors (Actor|GetAllActorsOfClass "/Game/exter/Blueprint/BP_ArenaTriggerErwan.BP_ArenaTriggerErwan_C"))
  (if (== (Utilities|Array|Length _outactors) 1)
    (for _array_element _outactors
      (LocalVariables|SetArenaErwan _array_element)
      (if (Variables|/Game/exter/Blueprint/BP_ArenaTriggerErwan.BP_ArenaTriggerErwan_C|GetIsArenaActive _array_element)
        (Default|DecrementEnemies (LocalVariables|GetArenaErwan) self)
        (Default|ArenaFinished (LocalVariables|GetArenaErwan))))))