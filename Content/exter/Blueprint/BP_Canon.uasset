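; BP_Canon is an automatic cannon that repeatedly fires BP_Melted_Caramel_Ball actors.
; BeginPlay attaches a fire effect to the fuse (Meche), then enables shooting, after an optional random delay that staggers its start.
; Tick drives a Delay of CanonCooldown as a repeating timer, then spawns a ball offset up and along the mesh's right vector, with an explosion effect.
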(event EventBeginPlay
  (Effects|SpawnEmitterAttached "/Game/StarterContent/Particles/P_Fire.P_Fire" (Variables|Default|Getmeche) "None" "0, 0, 0" "0, 0, 0" "0.200000,0.200000,0.100000" "KeepRelativeOffset" false)
  (if (Variables|Default|GetrandomStart)
    (Utilities|FlowControl|Delay (* (Math|Random|RandomFloat) 2.0)))
  (Variables|Default|SetstartShoot true))

(event EventTick
  (params (DeltaSeconds :type Float%20%28single-precision%29))
  (bind _staticmeshcomponent (Variables|Debug|GetStaticMeshComponent))
  (if (Variables|Default|GetstartShoot)
    (Utilities|FlowControl|Delay (Variables|Default|GetCanonCooldown))
    (Game|SpawnActorfromClass "/Game/exter/Blueprint/BP_Melted_Caramel_Ball.BP_Melted_Caramel_Ball_C" (Math|Transform|MakeTransform (+ (+ (Transformation|GetWorldLocation _staticmeshcomponent) "0, 0,50.000000") (* (Math|Vector|GetRightVector _staticmeshcomponent) 2.1e+02)) (Transformation|GetWorldRotation _staticmeshcomponent)) "Undefined" 0 0)
    (Effects|SpawnEmitterAttached "/Game/StarterContent/Particles/P_Explosion.P_Explosion" (Variables|Default|GetScene) "None")))

(fn ConstructionScript)