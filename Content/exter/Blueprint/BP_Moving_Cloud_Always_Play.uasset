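; Moving cloud actor that starts travelling along its spline as soon as play begins.
; The MovePlatform timeline has its looping set by Loop and its play rate divided by Time to control the trip duration.
; Each update scales the TravelDistance track by spline length and moves the static mesh to that local-space point, without sweep.
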(event EventBeginPlay
  (bind _moveplatform (Variables|Default|GetmovePlatform))
  (Components|Timeline|SetLooping _moveplatform (Variables|Default|Getloop))
  (Components|Timeline|SetPlayRate _moveplatform (/ (Components|Animation|GetPlayRate _moveplatform) (Variables|Default|Gettime)))
  (bind _traveldistance (Timeline|movePlatform Play)
    (:Update
      (Transformation|SetRelativeLocation (Variables|Default|GetStaticMesh) (Spline|GetLocationatDistanceAlongSpline (Variables|Default|GetSpline) (* _traveldistance (Spline|GetSplineLength (Variables|Default|GetSpline))) "Local") false false))))

(fn ConstructionScript)