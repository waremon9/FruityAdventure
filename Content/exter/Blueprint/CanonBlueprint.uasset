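; Cannon actor that repeatedly fires BouleDeCaramelEnFusion (molten caramel ball) actors.
; BeginPlay enables shooting, first waiting a random delay of up to two seconds when RandomStart is set.
; Tick drives a Delay of CanonCooldown to pace shots while shooting is enabled.
; Each ball spawns raised and offset along the mesh's right vector, matching the mesh's rotation.
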(event EventBeginPlay
  (if (Variables|Default|GetrandomStart)
    (Utilities|FlowControl|Delay (* (Math|Random|RandomFloat) 2.0)))
  (Variables|Default|SetstartShoot true))

(event EventTick
  (params (DeltaSeconds :type Float%20%28single-precision%29))
  (bind _staticmeshcomponent (Variables|Debug|GetStaticMeshComponent))
  (if (Variables|Default|GetstartShoot)
    (Utilities|FlowControl|Delay (Variables|Default|GetCanonCooldown))
    (Game|SpawnActorfromClass "/Game/exter/Blueprint/BouleDeCaramelEnFusion.BouleDeCaramelEnFusion_C" (Math|Transform|MakeTransform (+ (+ (Transformation|GetWorldLocation _staticmeshcomponent) "0, 0,50.000000") (* (Math|Vector|GetRightVector _staticmeshcomponent) 2.1e+02)) (Transformation|GetWorldRotation _staticmeshcomponent)) "Undefined" 0 0)))

(fn ConstructionScript)