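; Arena trigger that, on player overlap, spawns twenty BP_Goombagada on random clouds and starts a looping timer dropping one random cloud per second.
; BeginPlay caches every BP_Cloud4m and its location so ResetPlatform can restore them once all have fallen.
; Reset destroys leftover enemies and re-enables the trigger only if any remained.
; DecrementEnemies tracks removals; ArenaFinished resets platforms and starts CloudMoves when none remain.
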(event OnComponentBeginOverlap(CollisionComponent)
  (params (OverlappedComponent :type Primitive%20Component%20Object%20Reference) (OtherActor :type Actor%20Object%20Reference) (OtherComp :type Primitive%20Component%20Object%20Reference) (OtherBodyIndex :type Integer) (bFromSweep :type Boolean) (SweepResult :type Hit%20Result%20Structure%20%28by%20ref%29))
  (Utilities|Casting|CastToThirdPersonCharacter OtherActor)
  (for _index (range 0 19)
    (CallFunction|SpawnEnnemies))
  (Variables|Default|SetIsArenaActive true)
  (bind _returnvalue (Utilities|Time|SetTimerbyEvent (delegate Custom|PlateformFallDown) 1.0 true))
  (Variables|Default|SetTimerHandler _returnvalue)
  (Utilities|FlowControl|Delay 1.0)
  (Collision|SetCollisionEnabled (Variables|Default|GetCollisionComponent) "NoCollision"))

(event Custom|PlateformFallDown
  (bind _clouds (Variables|Default|GetClouds))
  (bind _output_get (Variables|Default|SetTempCloud (.OutItem (Utilities|Array|Random (Variables|Default|GetClouds)))))
  (Default|FallingDown _output_get)
  (Utilities|Array|RemoveItem _clouds (Variables|Default|GetTempCloud))
  (if (<= (Utilities|Array|Length _clouds) 0)
    (CallFunction|ResetPlatform)))

(event Custom|ResetPlatform
  (bind _enemies (Variables|Default|GetEnemies))
  (bind _enemies_2 (Variables|Default|GetEnemies))
  (Utilities|FlowControl|Delay 3.0)
  (Utilities|Time|ClearandInvalidateTimerbyHandle (Variables|Default|GetTimerHandler))
  (Utilities|Array|Clear (Variables|Default|GetClouds))
  (Variables|Default|SetClouds (Variables|Default|GetTempClouds))
  (Variables|Default|SetIsArenaActive false)
  (for (_array_element _array_index) (Variables|Default|GetClouds)
    (for (_array_element_2 _array_index_2) (Variables|Default|GetPlatformsVector)
      (Math|Integer|CompareInt _array_index _array_index_2
        (:==
          (Transformation|SetWorldLocation (Variables|/Script/Engine.StaticMeshActor|GetStaticMeshComponent _array_element) _array_element_2 false false)
          (Rendering|SetVisibility (Variables|/Script/Engine.StaticMeshActor|GetStaticMeshComponent _array_element) true false)
          (Collision|SetCollisionEnabled (Variables|/Script/Engine.StaticMeshActor|GetStaticMeshComponent _array_element) "QueryAndPhysics")
          (Rendering|Material|SetMaterial (Variables|/Script/Engine.StaticMeshActor|GetStaticMeshComponent _array_element) 0 "/Game/Platformer/Materials/M_Cloud.M_Cloud")))))
  (if (!= (Utilities|Array|Length (Variables|Default|GetEnemies)) 0)
    (Collision|SetCollisionEnabled (Variables|Default|GetCollisionComponent) "QueryAndPhysics")
    (for _array_element_3 _enemies
      (Actor|DestroyActor _array_element_3))
    (Utilities|Array|Clear _enemies)
    (else
      (for _array_element_4 _enemies_2
        (Actor|DestroyActor _array_element_4))
      (Utilities|Array|Clear _enemies_2))))

(event EventBeginPlay
  (Variables|Default|SetIsArenaActive false)
  (bind _outactors (Actor|GetAllActorsOfClass "/Game/exter/Blueprint/BP_Cloud4m.BP_Cloud4m_C"))
  (bind _output_get (Variables|Default|SetClouds _outactors))
  (Variables|Default|SetTempClouds _output_get)
  (for _array_element _output_get
    (Utilities|Array|Add (Variables|Default|GetPlatformsVector) (Transformation|GetWorldLocation (Variables|/Script/Engine.StaticMeshActor|GetStaticMeshComponent _array_element)))))

(fn ConstructionScript)

(fn SpawnEnnemies
  ;[1 1 1] Spawn enemies when the arena start
  (bind _returnvalue (AI|SpawnAIFromClass "/Game/exter/Blueprint/BP_Goombagada.BP_Goombagada_C" 0 (+ (Transformation|GetWorldLocation (Variables|/Script/Engine.StaticMeshActor|GetStaticMeshComponent (.OutItem (Utilities|Array|Random (Variables|Default|GetClouds))))) "0, 0,100.000000") "0, 0, 0" false 0))
  (bind _asbp_goombagada (Utilities|Casting|CastToBP_Goombagada _returnvalue))
  (Utilities|Array|Add (Variables|Default|GetEnemies) _asbp_goombagada))

(fn DecrementEnemies
  (params (Enemy :type BP%20Goombagada%20Object%20Reference))
  ;[1 1 1] Decrement the enemies array to find out if there are any enemies remaining
  (for _array_element (Variables|Default|GetEnemies)
    (bind _output_get (LocalVariables|SettempEnemy _array_element))
    (if (== _output_get Enemy)
      (Utilities|Array|RemoveItem (Variables|Default|GetEnemies) (LocalVariables|GettempEnemy)))))

(fn ArenaFinished
  ;[1 1 1] If there no more enemies then reset all platforms
  (if (== (Utilities|Array|Length (Variables|Default|GetEnemies)) 0)
    (CallFunction|ResetPlatform)
    (Default|Start (Variables|Default|GetCloudMoves))))