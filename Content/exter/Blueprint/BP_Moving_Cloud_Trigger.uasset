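; Moving cloud platform that travels along a spline when the third-person character enters its trigger box or Start is called.
; Type selects the default or special timeline, which runs at a rate set by Time, optionally looping, and maps its output to distance along the spline.
; A Started flag blocks retriggering until the timeline finishes.
; ResetCloud stops that timeline, teleports the mesh to its BeginPlay location and clears the flag.
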(event OnComponentBeginOverlap(Box)
  (params (OverlappedComponent :type Primitive%20Component%20Object%20Reference) (OtherActor :type Actor%20Object%20Reference) (OtherComp :type Primitive%20Component%20Object%20Reference) (OtherBodyIndex :type Integer) (bFromSweep :type Boolean) (SweepResult :type Hit%20Result%20Structure%20%28by%20ref%29))
  (bind _specialmove1 (Variables|Default|GetSpecialMove1))
  (bind _moveplatformdefault (Variables|Default|GetmovePlatformDefault))
  (bind _spline (Variables|Default|GetSpline))
  (Utilities|Casting|CastToThirdPersonCharacter OtherActor)
  (if (not (Variables|Default|Getstarted))
    (Variables|Default|Setstarted true)
    (switch int (Variables|Default|Gettype)
      (:Default
        (Components|Timeline|SetLooping _moveplatformdefault (Variables|Default|Getloop) :!label _label)
        (Components|Timeline|SetPlayRate _moveplatformdefault (/ 1.0 (Variables|Default|Gettime)))
        (bind _traveldistance (Timeline|movePlatformDefault PlayFromStart)
          (:Update
            (Variables|Default|SettravelDist _traveldistance)
            (Transformation|SetRelativeLocation (Variables|Default|GetStaticMesh) (Spline|GetLocationatDistanceAlongSpline _spline (* (Spline|GetSplineLength _spline) (Variables|Default|GettravelDist)) "Local") false false :!label _label_2))
          (:Finished
            (Variables|Default|Setstarted false :!label _label_3))))
      (:0
        (goto _label))
      (:1
        (Components|Timeline|SetLooping _specialmove1 (Variables|Default|Getloop))
        (Components|Timeline|SetPlayRate _specialmove1 (/ 1.0 (Variables|Default|Gettime)))
        (bind _traveldistance_2 (Timeline|SpecialMove1 PlayFromStart)
          (:Update
            (Variables|Default|SettravelDist _traveldistance_2)
            (goto _label_2))
          (:Finished
            (goto _label_3)))))))

(event Custom|Start
  (bind _specialmove1 (Variables|Default|GetSpecialMove1))
  (bind _moveplatformdefault (Variables|Default|GetmovePlatformDefault))
  (bind _spline (Variables|Default|GetSpline))
  (if (not (Variables|Default|Getstarted))
    (Variables|Default|Setstarted true)
    (switch int (Variables|Default|Gettype)
      (:Default
        (Components|Timeline|SetLooping _moveplatformdefault (Variables|Default|Getloop) :!label _label)
        (Components|Timeline|SetPlayRate _moveplatformdefault (/ 1.0 (Variables|Default|Gettime)))
        (bind _traveldistance (Timeline|movePlatformDefault PlayFromStart)
          (:Update
            (Variables|Default|SettravelDist _traveldistance)
            (Transformation|SetRelativeLocation (Variables|Default|GetStaticMesh) (Spline|GetLocationatDistanceAlongSpline _spline (* (Spline|GetSplineLength _spline) (Variables|Default|GettravelDist)) "Local") false false :!label _label_2))
          (:Finished
            (Variables|Default|Setstarted false :!label _label_3))))
      (:0
        (goto _label))
      (:1
        (Components|Timeline|SetLooping _specialmove1 (Variables|Default|Getloop))
        (Components|Timeline|SetPlayRate _specialmove1 (/ 1.0 (Variables|Default|Gettime)))
        (bind _traveldistance_2 (Timeline|SpecialMove1 PlayFromStart)
          (:Update
            (Variables|Default|SettravelDist _traveldistance_2)
            (goto _label_2))
          (:Finished
            (goto _label_3)))))))

(event Custom|ResetCloud
  (switch int (Variables|Default|Gettype)
    (:Default
      (Audio|Components|Audio|Stop (Variables|Default|GetmovePlatformDefault) :!label _label))
    (:0
      (goto _label))
    (:1
      (Audio|Components|Audio|Stop (Variables|Default|GetSpecialMove1))))
  (Transformation|SetWorldLocation (Variables|Default|GetStaticMesh) (Variables|Default|GetStartLocation) false true)
  (Variables|Default|Setstarted false))

(event EventBeginPlay
  (Variables|Default|SetStartLocation (Transformation|GetWorldLocation (Variables|Default|GetStaticMesh))))

(fn ConstructionScript)