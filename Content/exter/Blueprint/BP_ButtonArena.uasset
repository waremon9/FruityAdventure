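; BP_ButtonArena is an interactable button in an ordered sequence puzzle, accepting the Interact input while its trigger box is overlapped.
; Pressed with its Previous button active or unset, it turns green, plays an effect and increments NbButtonOn on BP_Trigger_Killian.
; Pressed out of order, it zeroes that count and recurses through the Previous chain, turning active buttons red, then the chain grey after a delay.
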(event OnComponentBeginOverlap(Box)
  (params (OverlappedComponent :type Primitive%20Component%20Object%20Reference) (OtherActor :type Actor%20Object%20Reference) (OtherComp :type Primitive%20Component%20Object%20Reference) (OtherBodyIndex :type Integer) (bFromSweep :type Boolean) (SweepResult :type Hit%20Result%20Structure%20%28by%20ref%29))
  (Input|EnableInput (Game|GetPlayerController 0)))

(event OnComponentEndOverlap(Box)
  (params (OverlappedComponent :type Primitive%20Component%20Object%20Reference) (OtherActor :type Actor%20Object%20Reference) (OtherComp :type Primitive%20Component%20Object%20Reference) (OtherBodyIndex :type Integer))
  (Input|DisableInput (Game|GetPlayerController 0)))

(event EventBeginPlay)

(event Input|ActionEvents|InputActionInteract
  (params (Key :type Key%20Structure :default "None"))
  (bind _previous (Variables|Default|GetPrevious))
  (bind _niagara (Variables|Default|GetNiagara))
  (bind _niagara_2 (Variables|Default|GetNiagara))
  (:Pressed
    (if (Utilities|IsValid _previous)
      (if (Variables|BP_ButtonArena_C|GetActivated _previous)
        (bind _returnvalue (Rendering|Material|CreateDynamicMaterialInstance (Variables|Default|GetCube) 0 "/Game/exter/Blueprint/ButtonOn.ButtonOn" "None" :!class /Script/Engine.PrimitiveComponent :!label _label))
        (Rendering|Material|SetVectorParameterValue _returnvalue "ActivationColor" (Math|Color|MakeColor 0.0 1.0 0.0) :!class /Script/Engine.MaterialInstanceDynamic)
        (if (not (Variables|Default|GetActivated))
          (Variables|Default|SetActivated true)
          (bind _returnvalue_2 (Actor|GetActorOfClass "/Game/exter/Blueprint/BP_Trigger_Killian.BP_Trigger_Killian_C"))
          (bind _result (Math|Integer|IncrementInt (Variables|/Game/exter/Blueprint/BP_Trigger_Killian.BP_Trigger_Killian_C|GetNbButtonOn _returnvalue_2))
            (:%20%20
              (Variables|/Game/exter/Blueprint/BP_Trigger_Killian.BP_Trigger_Killian_C|SetNbButtonOn _returnvalue_2 _result)
              (Class|NiagaraComponent|SetAsset _niagara_2 "/Game/Stylized_VFX_StPack/Particles/UPDATE_1_2/P_Classic_Hit_03.P_Classic_Hit_03")
              (Components|Activation|Activate _niagara_2 true))))
        (else
          (Variables|Default|SetActivated true)
          (Class|NiagaraComponent|SetAsset _niagara "/Game/Stylized_VFX_StPack/Particles/UPDATE_1_2/P_Snaking_Hit_03.P_Snaking_Hit_03")
          (Components|Activation|Activate _niagara true)
          (CallFunction|Desactive)
          (bind _returnvalue_3 (Actor|GetActorOfClass "/Game/exter/Blueprint/BP_Trigger_Killian.BP_Trigger_Killian_C"))
          (Variables|/Game/exter/Blueprint/BP_Trigger_Killian.BP_Trigger_Killian_C|SetNbButtonOn _returnvalue_3 0)
          (Utilities|FlowControl|Delay 2.7)
          (CallFunction|ChangeMat)))
      (else
        (goto _label)))))

(fn ConstructionScript)

(fn Desactive
  (bind _previous (Variables|Default|GetPrevious))
  (if (Variables|Default|GetActivated)
    (Variables|Default|SetActivated false)
    (bind _returnvalue (Rendering|Material|CreateDynamicMaterialInstance (Variables|Default|GetCube) 0 "/Game/exter/Blueprint/ButtonOn.ButtonOn" "None" :!class /Script/Engine.PrimitiveComponent))
    (Rendering|Material|SetVectorParameterValue _returnvalue "ActivationColor" (Math|Color|MakeColor 1.0 0.0 0.0) :!class /Script/Engine.MaterialInstanceDynamic))
  (if (Utilities|IsValid _previous)
    (CallFunction|Desactive _previous)))

(fn ChangeMat
  (bind _previous (Variables|Default|GetPrevious))
  (Rendering|Material|CreateDynamicMaterialInstance (Variables|Default|GetCube) 0 "/Game/Stylized_VFX_StPack/MAP/MAP_Materials/MI_Grey.MI_Grey" "None" :!class /Script/Engine.PrimitiveComponent)
  (if (Utilities|IsValid _previous)
    (CallFunction|ChangeMat _previous)))