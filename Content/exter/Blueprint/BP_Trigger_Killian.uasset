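; BP_Trigger_Killian is a trigger that runs the Killian arena encounter until its final button is activated.
; Box overlap shows the KillianAreneHUD, passes it a self reference, and starts a looping timer spawning scaled-up asteroid projectiles at random positions overhead.
; While active, Tick polls ButtonFinal; once activated, it removes the HUD, calls DestroyDoor, then after a delay destroys the door and itself.
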(event OnComponentBeginOverlap(Box)
  (params (OverlappedComponent :type Primitive%20Component%20Object%20Reference) (OtherActor :type Actor%20Object%20Reference) (OtherComp :type Primitive%20Component%20Object%20Reference) (OtherBodyIndex :type Integer) (bFromSweep :type Boolean) (SweepResult :type Hit%20Result%20Structure%20%28by%20ref%29))
  (if (not (Variables|Default|GetActivated))
    (Variables|Default|SetActivated true)
    (Utilities|FlowControl|Sequence
      (:then_0
        (bind _returnvalue (UserInterface|CreateWidget "/Game/exter/HUD/KillianAreneHUD.KillianAreneHUD_C"))
        (bind _output_get (Variables|Default|Sethud _returnvalue))
        (UserInterface|Viewport|AddtoViewport _output_get 0))
      (:then_1
        (Variables|/Game/exter/HUD/KillianAreneHUD.KillianAreneHUD_C|SetTriggerKillian (Variables|Default|Gethud) self))
      (:then_2
        (Utilities|Time|SetTimerbyEvent (delegate Custom|SpawnAsteroide) 1.0 true)))))

(event Custom|SpawnAsteroide
  (Game|SpawnActorfromClass "/Game/exter/Blueprint/BP_Asteroid_Projectile.BP_Asteroid_Projectile_C" (Math|Transform|MakeTransform (Math|Vector|MakeVector (Math|Random|RandomFloatinRange -3.8e+03 5e+02) (Math|Random|RandomFloatinRange 3.9e+03 8.1e+03) 5e+03) "-90.000000, 0, 0" "10.000000,10.000000,10.000000") "Undefined" 0 false 1e+03 1 0))

(event EventBeginPlay)

(event Collision|EventActorBeginOverlap
  (params (OtherActor :type Actor%20Object%20Reference)))

(event EventTick
  (params (DeltaSeconds :type Float%20%28single-precision%29))
  (bind _door (Variables|Default|GetDoor))
  (if (Variables|Default|GetActivated)
    (if (Variables|/Game/exter/Blueprint/BP_ButtonArena.BP_ButtonArena_C|GetActivated (Variables|Default|GetButtonFinal))
      (Variables|Default|SetActivated false)
      (Widget|RemovefromParent (Variables|Default|Gethud))
      (Default|DestroyDoor _door)
      (Utilities|FlowControl|Delay 5.0)
      (Actor|DestroyActor _door)
      (Actor|DestroyActor))))

(fn ConstructionScript)