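; BouncyPlatform_BP is a bouncy platform that launches the player upward with a boing sound and a brief squash.
; Box overlap events toggle a flag that Tick polls, launching player character 0 by LaunchPower with Z override, whichever actor overlaps.
; Each overlapping tick also replays the sound and multiplies the mesh scale, which is divided back after a short Delay, so repeated ticks can compound the squash.
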(event OnComponentBeginOverlap(Box)
  (params (OverlappedComponent :type Primitive%20Component%20Object%20Reference) (OtherActor :type Actor%20Object%20Reference) (OtherComp :type Primitive%20Component%20Object%20Reference) (OtherBodyIndex :type Integer) (bFromSweep :type Boolean) (SweepResult :type Hit%20Result%20Structure%20%28by%20ref%29))
  (Variables|Default|Setoverlap true))

(event OnComponentEndOverlap(Box)
  (params (OverlappedComponent :type Primitive%20Component%20Object%20Reference) (OtherActor :type Actor%20Object%20Reference) (OtherComp :type Primitive%20Component%20Object%20Reference) (OtherBodyIndex :type Integer))
  (Variables|Default|Setoverlap false))

(event EventTick
  (params (DeltaSeconds :type Float%20%28single-precision%29))
  (bind _returnvalue (Math|Vector|MakeVector 1.2 1.2 0.7))
  (bind _staticmeshcomponent (Variables|Debug|GetStaticMeshComponent))
  (bind _returnvalue_2 (Transformation|GetWorldScale _staticmeshcomponent))
  (if (Variables|Default|Getoverlap)
    (Character|LaunchCharacter (Game|GetPlayerCharacter 0) (Variables|Default|GetLaunchPower) false true)
    (Audio|PlaySound2D "/Game/exter/Audio/A_Boing.A_Boing" 1.0 1.0 0.0 0 0)
    (Transformation|SetWorldScale3D _staticmeshcomponent (* _returnvalue_2 _returnvalue))
    (Utilities|FlowControl|Delay 0.1)
    (Transformation|SetWorldScale3D _staticmeshcomponent (/ _returnvalue_2 _returnvalue))))

(fn ConstructionScript)