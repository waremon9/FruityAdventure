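; Checkpoint actor that sets the player's respawn point the first time a ThirdPersonCharacter overlaps it.
; A boolean guard limits activation to once, playing a sound, switching the mesh to a blue plastic material and activating a Niagara effect.
; The Scene component's world location, without its rotation, becomes the SpawnLocation transform in ThirdPersonGameMode.
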(event Collision|EventActorBeginOverlap
  (params (OtherActor :type Actor%20Object%20Reference))
  (Utilities|Casting|CastToThirdPersonCharacter OtherActor)
  (if (not (Variables|Default|GetCheckpointEnabled))
    (Variables|Default|SetCheckpointEnabled true)
    (Audio|PlaySound2D "/Game/exter/Audio/A_Checkpoint.A_Checkpoint" 1.0 1.0 0.0 0 0)
    (Rendering|Material|CreateDynamicMaterialInstance (Variables|Default|GetStaticMesh1) 0 "/Game/Platformer/Materials/M_Plastic_blue_Inst.M_Plastic_blue_Inst" "None" :!class /Script/Engine.PrimitiveComponent)
    (bind _asthird_person_game_mode (Utilities|Casting|CastToThirdPersonGameMode (Game|GetGameMode)))
    (Variables|/Game/ThirdPersonBP/Blueprints/ThirdPersonGameMode.ThirdPersonGameMode_C|SetspawnLocation _asthird_person_game_mode (Math|Conversions|ToTransform(Vector) (Transformation|GetWorldLocation (Variables|Default|GetScene))))
    (Components|Activation|Activate (Variables|Default|GetNiagara) true)))

(fn ConstructionScript)