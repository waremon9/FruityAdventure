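; BP_Gun is a turret that rotates every tick to face the player character's mesh.
; Any overlap with its Sphere starts a looping cooldown timer, and end overlap clears the stored timer handle.
; Each timer firing spawns a BP_Gun_Bullet at the Scene component and applies an impulse toward a point above the player mesh's origin, scaled by distance.
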(event OnComponentBeginOverlap(Sphere)
  (params (OverlappedComponent :type Primitive%20Component%20Object%20Reference) (OtherActor :type Actor%20Object%20Reference) (OtherComp :type Primitive%20Component%20Object%20Reference) (OtherBodyIndex :type Integer) (bFromSweep :type Boolean) (SweepResult :type Hit%20Result%20Structure%20%28by%20ref%29))
  (bind _returnvalue (Utilities|Time|SetTimerbyEvent (delegate Custom|Shoot) (Variables|Default|GetshootCooldown) true))
  (Variables|Default|Settimerhandler _returnvalue))

(event OnComponentEndOverlap(Sphere)
  (params (OverlappedComponent :type Primitive%20Component%20Object%20Reference) (OtherActor :type Actor%20Object%20Reference) (OtherComp :type Primitive%20Component%20Object%20Reference) (OtherBodyIndex :type Integer))
  (Utilities|Time|ClearandInvalidateTimerbyHandle (Variables|Default|Gettimerhandler)))

(event Custom|Shoot
  (bind _returnvalue (Game|SpawnActorfromClass "/Game/exter/Blueprint/BP_Gun_Bullet.BP_Gun_Bullet_C" (Math|Conversions|ToTransform(Vector) (Transformation|GetWorldLocation (Variables|Default|GetScene))) "Undefined" 0 0))
  (Physics|AddImpulse (Variables|/Game/exter/Blueprint/BP_Gun_Bullet.BP_Gun_Bullet_C|GetSphere _returnvalue) (* (- (+ (Transformation|GetWorldLocation (Variables|/Script/Engine.Character|GetMesh (Game|GetPlayerCharacter 0))) "0, 0,250.000000") (Transformation|GetWorldLocation (Variables|Default|GetScene))) 0.5) "None" false))

(event EventTick
  (params (DeltaSeconds :type Float%20%28single-precision%29))
  (Transformation|SetActorRotation (Math|Rotator|FindLookatRotation (Transformation|GetWorldLocation (Variables|Default|GetStaticMesh)) (Transformation|GetWorldLocation (Variables|/Script/Engine.Character|GetMesh (Game|GetPlayerCharacter 0))))))

(fn ConstructionScript)