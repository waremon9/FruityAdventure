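; BP_Fruit_Parent is the base collectible fruit pickup, which spins constantly and is collected when the ThirdPersonCharacter overlaps it.
; Collection notifies the character via GetFruit, deactivates the pickup particle, plays a sound, disables collision and raises the fruit.
; After rising, Tick steps it from its saved position toward the player's current location over a fixed number of frames, then destroys it.
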(event Custom|collect
  (bind _defaultsceneroot (Variables|Default|GetDefaultSceneRoot))
  (bind _returnvalue (Transformation|GetWorldLocation _defaultsceneroot))
  ;[1 1 1] on contact, coins start going up
  (bind _asthird_person_character (Utilities|Casting|CastToThirdPersonCharacter (Game|GetPlayerCharacter 0)))
  (Default|GetFruit _asthird_person_character)
  (Components|Activation|Deactivate (Variables|Default|GetpickupParticle))
  (Audio|PlaySound2D "/Game/exter/Audio/A_Pickup.A_Pickup" 1.0 1.0 0.0 0 0)
  (Collision|SetActorEnableCollision false)
  (Components|MoveComponentTo _defaultsceneroot (+ _returnvalue "0, 0,500.000000") "0, 0, 0" false false (Variables|Default|GetTimeToMoveUp) false)
  (Variables|Default|SetFollowPlayer true)
  (Variables|Default|SetOriginalLocation _returnvalue))

(event Collision|EventActorBeginOverlap
  (params (OtherActor :type Actor%20Object%20Reference))
  (Utilities|Casting|CastToThirdPersonCharacter OtherActor)
  (CallFunction|Collect))

(event EventTick
  (params (DeltaSeconds :type Float%20%28single-precision%29))
  (bind _i (Variables|Default|Geti))
  (bind _originallocation (Variables|Default|GetOriginalLocation))
  (bind _gotoplayernbofpoint (Variables|Default|GetGoToPlayerNbOfPoint))
  ;[1 1 1] Rotation
  (Transformation|AddActorLocalRotation "0,5.000000, 0" false false)
  ;[1 1 1] Coin follow player then touch him and dissapear
  (if (Variables|Default|GetFollowPlayer)
    (if (< _i _gotoplayernbofpoint)
      (Transformation|SetActorLocation (+ _originallocation (* (/ (- (Transformation|GetActorLocation (Game|GetPlayerCharacter 0)) _originallocation) (Math|Conversions|ToFloat(Integer) _gotoplayernbofpoint)) (Math|Conversions|ToFloat(Integer) _i))) false false)
      (Math|Integer|IncrementInt _i)
      (else
        (Actor|DestroyActor)))))

(fn ConstructionScript)