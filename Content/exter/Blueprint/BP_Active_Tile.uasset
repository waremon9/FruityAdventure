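; BP_Active_Tile is a floor-tile style toggle that flips its Activated state whenever the ThirdPersonCharacter begins overlapping its Box.
; Each toggle swaps the mesh material between red wood for inactive and yellow wood for active.
; FinishEvent turns the tile green and sets Finished, which blocks further toggling.
; The resetTile event clears both flags and restores the red material.
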(event OnComponentBeginOverlap(Box)
  (params (OverlappedComponent :type Primitive%20Component%20Object%20Reference) (OtherActor :type Actor%20Object%20Reference) (OtherComp :type Primitive%20Component%20Object%20Reference) (OtherBodyIndex :type Integer) (bFromSweep :type Boolean) (SweepResult :type Hit%20Result%20Structure%20%28by%20ref%29))
  (Utilities|Casting|CastToThirdPersonCharacter OtherActor)
  (if (not (Variables|Default|GetFinished))
    (if (Variables|Default|GetActivated)
      (Variables|Default|SetActivated false)
      (Rendering|Material|SetMaterial (Variables|Debug|GetStaticMeshComponent) 0 "/Game/Platformer/Materials/M_Wood_Red.M_Wood_Red")
      (else
        (Variables|Default|SetActivated true)
        (Rendering|Material|SetMaterial (Variables|Debug|GetStaticMeshComponent) 0 "/Game/Platformer/Materials/M_Wood_Yellow.M_Wood_Yellow")))))

(event Custom|FinishEvent
  (Variables|Default|SetFinished true)
  (Rendering|Material|SetMaterial (Variables|Debug|GetStaticMeshComponent) 0 "/Game/Platformer/Materials/M_Wood_Green.M_Wood_Green"))

(event Custom|resetTile
  (Variables|Default|SetActivated false)
  (Variables|Default|SetFinished false)
  (Rendering|Material|SetMaterial (Variables|Debug|GetStaticMeshComponent) 0 "/Game/Platformer/Materials/M_Wood_Red.M_Wood_Red"))

(fn ConstructionScript)