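; A disappearing cloud platform that sinks and vanishes after the ThirdPersonCharacter touches it, then respawns.
; On overlap, the trigger box turns off and MoveComponentTo lowers the mesh over 1.5 seconds, using the stored world start location as a relative-space target.
; The actor then loses mesh collision and hides.
; After a delay, it teleports the mesh back, restores both collisions and reappears.
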(event OnComponentBeginOverlap(Box)
  (params (OverlappedComponent :type Primitive%20Component%20Object%20Reference) (OtherActor :type Actor%20Object%20Reference) (OtherComp :type Primitive%20Component%20Object%20Reference) (OtherBodyIndex :type Integer) (bFromSweep :type Boolean) (SweepResult :type Hit%20Result%20Structure%20%28by%20ref%29))
  (Utilities|Casting|CastToThirdPersonCharacter OtherActor)
  (Collision|SetCollisionEnabled (Variables|Default|GetBox) "NoCollision")
  (Components|MoveComponentTo (Variables|Debug|GetStaticMeshComponent) (- (Variables|Default|GetOriginaLocation) "0, 0,200.000000") "0, 0, 0" false false 1.5 false)
  (Collision|SetCollisionEnabled (Variables|Debug|GetStaticMeshComponent) "NoCollision")
  (Rendering|SetActorHiddenInGame true)
  (Utilities|FlowControl|Delay 4.0)
  (Transformation|SetWorldLocation (Variables|Debug|GetStaticMeshComponent) (Variables|Default|GetOriginaLocation) false true)
  (Collision|SetCollisionEnabled (Variables|Debug|GetStaticMeshComponent) "QueryAndPhysics")
  (Collision|SetCollisionEnabled (Variables|Default|GetBox) "QueryAndPhysics")
  (Rendering|SetActorHiddenInGame false))

(event EventBeginPlay
  (Variables|Default|SetOriginaLocation (Transformation|GetWorldLocation (Variables|Debug|GetStaticMeshComponent))))

(fn ConstructionScript)