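; BP_Arena_Trigger_Thomas is an arena entry trigger that seals the player in by raising a set of doors.
; When a ThirdPersonCharacter overlaps its collision component, every actor in the Door array becomes visible and solid, and the trigger disables its own collision so it fires once.
; The resetEntry event reverses this, hiding the doors, removing their collision and re-arming the trigger.
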(event OnComponentBeginOverlap(CollisionComponent)
  (params (OverlappedComponent :type Primitive%20Component%20Object%20Reference) (OtherActor :type Actor%20Object%20Reference) (OtherComp :type Primitive%20Component%20Object%20Reference) (OtherBodyIndex :type Integer) (bFromSweep :type Boolean) (SweepResult :type Hit%20Result%20Structure%20%28by%20ref%29))
  (Utilities|Casting|CastToThirdPersonCharacter OtherActor)
  (for _array_element (Variables|Default|GetDoor)
    (Rendering|SetVisibility (Variables|/Script/Engine.StaticMeshActor|GetStaticMeshComponent _array_element) true false)
    (Collision|SetCollisionEnabled (Variables|/Script/Engine.StaticMeshActor|GetStaticMeshComponent _array_element) "QueryAndPhysics"))
  (Collision|SetCollisionEnabled (Variables|Default|GetCollisionComponent) "NoCollision"))

(event Custom|resetEntry
  (for _array_element (Variables|Default|GetDoor)
    (Rendering|SetVisibility (Variables|/Script/Engine.StaticMeshActor|GetStaticMeshComponent _array_element) false false)
    (Collision|SetCollisionEnabled (Variables|/Script/Engine.StaticMeshActor|GetStaticMeshComponent _array_element) "NoCollision"))
  (Collision|SetCollisionEnabled (Variables|Default|GetCollisionComponent) "QueryAndPhysics"))

(fn ConstructionScript)