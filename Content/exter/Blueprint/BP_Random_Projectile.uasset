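; BP_Random_Projectile is a projectile actor that travels in a straight line along a random direction.
; BeginPlay picks a random unit vector as its Direction.
; Each Tick moves the Sphere component by Direction times Speed times delta time, without sweeping, so movement does no collision checks along the path.
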(event EventBeginPlay
  (Variables|Default|SetDirection (Math|Random|RandomUnitVector)))

(event EventTick
  (params (DeltaSeconds :type Float%20%28single-precision%29))
  (Transformation|SetWorldLocation (Variables|Default|GetSphere) (+ (* (* (Variables|Default|GetDirection) (Variables|Default|GetSpeed)) DeltaSeconds) (Transformation|GetWorldLocation (Variables|Default|GetSphere))) false false))

(fn ConstructionScript)