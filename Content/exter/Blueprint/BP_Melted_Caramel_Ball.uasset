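; BP_Melted_Caramel_Ball is a hazard actor, apparently a projectile, that explodes on contact.
; Its Sphere destroys the actor on any hit, while overlapping a ThirdPersonCharacter calls that character's Hit before destroying it.
; The Destroyed event spawns an explosion particle at the actor and plays an attenuated explosion sound at the Sphere, so every removal gets the same effect.
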(event OnComponentBeginOverlap(Sphere)
  (params (OverlappedComponent :type Primitive%20Component%20Object%20Reference) (OtherActor :type Actor%20Object%20Reference) (OtherComp :type Primitive%20Component%20Object%20Reference) (OtherBodyIndex :type Integer) (bFromSweep :type Boolean) (SweepResult :type Hit%20Result%20Structure%20%28by%20ref%29))
  (bind _asthird_person_character (Utilities|Casting|CastToThirdPersonCharacter OtherActor))
  (Default|Hit _asthird_person_character)
  (Actor|DestroyActor))

(event OnComponentHit(Sphere)
  (params (HitComponent :type Primitive%20Component%20Object%20Reference) (OtherActor :type Actor%20Object%20Reference) (OtherComp :type Primitive%20Component%20Object%20Reference) (NormalImpulse :type Vector :default "0, 0, 0") (Hit :type Hit%20Result%20Structure%20%28by%20ref%29))
  (Actor|DestroyActor))

(event Custom|PlayParticle
  (Effects|SpawnEmitteratLocation "/Game/FXVarietyPack/Particles/P_ky_explosion.P_ky_explosion" (Transformation|GetActorLocation)))

(event EventDestroyed
  (CallFunction|PlayParticle)
  (Audio|PlaySoundatLocation "/Game/StarterContent/Audio/Explosion01.Explosion01" (Transformation|GetWorldLocation (Variables|Default|GetSphere)) "0, 0, 0" 0.5 1.0 0.0 "/Game/exter/Audio/ATT_Classic.ATT_Classic" 0 0))

(fn ConstructionScript)